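; BP_FinalDoor is a large double door in the medieval dungeon that opens on an Interact event unless IsLocked is set.
; A DoOnce gate starts a timeline that swings the right and left door meshes apart by lerping their relative yaw to opposite right angles.
; The wooden opening sound plays from the timeline's Update pin on every tick, located at the world origin rather than at the door.
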(event EventBeginPlay)

(event Collision|EventActorBeginOverlap
  (params (OtherActor :type Actor%20Object%20Reference)))

(event EventTick
  (params (DeltaSeconds :type Float%20%28single-precision%29)))

(event EventInteract
  (if (not (Variables|Default|GetIsLocked))
    (Utilities|FlowControl|DoOnce false
      (:Completed
        (bind _newtrack_0 (Timeline|Timeline Play)
          (:Update
            (Audio|PlaySoundatLocation "/Game/Audio/MetaSound/Audiosource/SFX/Play_Door_Wood_Open.Play_Door_Wood_Open" "0, 0, 0" "0, 0, 0" 1.0 1.0 0.0 0 0 0 0)
            (Transformation|SetRelativeRotation (Variables|Default|GetSM_DoorWay_Large_Door_Right) (Math|Rotator|MakeRotator 0.0 0.0 (Math|Float|Lerp 0.0 9e+01 _newtrack_0)) false false)
            (Transformation|SetRelativeRotation (Variables|Default|GetSM_DoorWay_Large_Door_Left) (Math|Rotator|MakeRotator 0.0 0.0 (Math|Float|Lerp 0.0 -9e+01 _newtrack_0)) false false)))))))

(fn ConstructionScript)